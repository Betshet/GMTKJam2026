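; BP_PathManager is an actor for generating paths of ground points and spline segments, though it is only partly implemented.
; SamplePoints splits the bounds box into equal slices along local X and picks one random, inset point per slice at the box top, in world space.
; TraceGround line-traces down with debug drawing and returns the hit plus an offset.
; GeneratePath, segment building and the acquire/release functions are empty stubs, so nothing connects these steps.
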(fn `AcquirePoint`
  (params (Index :type Integer))
  (returns (PointActor :type "Actor Object Reference"))
  (return null))

(fn `AcquireSpline`
  (params (Index :type Integer))
  (returns (SplineComp :type "SplineComponent Object Reference"))
  (return null))

(fn `BuildSegment`
  (params (Spline :type "SplineComponent Object Reference") (Start :type "Vector Structure") (End :type "Vector Structure") (SegmentIndex :type Integer)))

(fn `GeneratePath`
  (params (NumPoints :type Integer)))

(fn `ReleaseAll`)

(fn `SamplePoints`
  (params (NumPoints :type Integer))
  (returns (OutSampledPoints :type "Array of Vector Structure"))
  (locals (Sampled :type "Array of Vector Structure") (ExtentX :type "Float (double-precision)" :default 0.0) (ExtentY :type "Float (double-precision)" :default 0.0) (SliceWidth :type "Float (double-precision)") (Inset :type "Float (double-precision)") (ExtentZ :type "Float (double-precision)" :default 0.0))
  (bind _extenty (`local.ExtentY`))
  (bind _inset (`local.Inset`))
  (bind (_returnvalue_x _returnvalue_y _returnvalue_z) (`KismetMathLibrary.BreakVector` (`BoxComponent.GetScaledBoxExtent` (`self.PathPointsBounds`))))
  (`KismetArrayLibrary.Array_Clear` (`local.Sampled`))
  (set `local.ExtentX` _returnvalue_x)
  (set `local.ExtentY` _returnvalue_y)
  (set `local.ExtentZ` _returnvalue_z)
  (set `local.SliceWidth` (/ (* _returnvalue_x 2.0) (`local.NumPoints`)))
  (set `local.Inset` (* (`local.SliceWidth`) 0.15))
  (for _index (range (+ (`local.NumPoints`) 1))
    (bind _returnvalue (- (`local.ExtentX`) (* (`local.SliceWidth`) _index)))
    (`KismetArrayLibrary.Array_Add` (`local.Sampled`) (`KismetMathLibrary.TransformLocation` (`SceneComponent.K2_GetComponentToWorld` (`self.PathPointsBounds`)) (`KismetMathLibrary.MakeVector` (`KismetMathLibrary.RandomFloatInRange` (+ (- _returnvalue (`local.SliceWidth`)) _inset) (- _returnvalue _inset)) (`KismetMathLibrary.RandomFloatInRange` (* _extenty -1.0) _extenty) (`local.ExtentZ`)))))
  (return (`local.Sampled`)))

(fn `TraceGround`
  (params (At :type "Vector Structure"))
  (returns (Success :type Boolean) (GroundPoint :type "Vector Structure"))
  (bind (_outhit _returnvalue) (`KismetSystemLibrary.LineTraceSingle` :`Start` (+ At (0.0 0.0 100.0)) :`End` (- At (0.0 0.0 5000.0)) :`TraceChannel` "TraceTypeQuery1" :`DrawDebugType` "ForDuration" :`DrawTime` 1000.0))
  (return _returnvalue (+ (`.Location` (`GameplayStatics.BreakHitResult` _outhit)) (`KismetMathLibrary.MakeVector` 0.0 0.0 (`self.GroundOffset`)))))

(fn `UserConstructionScript`)